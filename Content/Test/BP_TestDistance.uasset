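; Test actor that scores how close the player is and how they are oriented toward it, and displays that score.
; A looping timer sums a clamped inverse distance and a weighted, normalized angle between the player capsule's and text's forward vectors.
; It writes the sum to a TextRender, then yaws the actor to face the player.
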(event Custom|CalculDistance
  (bind _distancetoplayer (CallFunction|CalculDistance (Transformation|GetActorLocation (Variables|Default|GetPlayer))))
  (bind _angle (CallFunction|CalculAngle))
  (Variables|Default|SetFinalScore (+ (/ _angle (Variables|Default|GetPoidDeAngle)) _distancetoplayer))
  (CallFunction|SetText (+ (/ _angle (Variables|Default|GetPoidDeAngle)) _distancetoplayer))
  (CallFunction|FacePlayer))

(event EventBeginPlay
  (bind _asbp_third_person_character (Utilities|Casting|CastToBP_ThirdPersonCharacter (Game|GetPlayerCharacter 0)))
  (Variables|Default|SetPlayer _asbp_third_person_character)
  (Utilities|Time|SetTimerbyEvent (delegate Custom|CalculDistance) 0.1 true))

(fn ConstructionScript)

(fn CalculDistance
  (params (PlayerLocation :type Vector))
  (bind _output_get (LocalVariables|SetDistance (Math|Float|Clamp(Float) (- 1.2 (/ (Math|Vector|Distance(Vector) PlayerLocation (Transformation|GetActorLocation)) (Variables|Default|GetMax))))))
  (return _output_get))

(fn SetText
  (params (DistanceToPlayer :type Float%20%28double-precision%29))
  (Rendering|Components|TextRender|SetText (Variables|Default|GetTextRender) (Utilities|Text|ToText(Float) DistanceToPlayer "HalfToEven")))

(fn FacePlayer
  (Transformation|SetActorRotation (Math|Rotator|MakeRotator 0.0 0.0 (.yaw (Math|Rotator|FindLookatRotation (Transformation|GetActorLocation) (Transformation|GetActorLocation (Variables|Default|GetPlayer)))))))

(fn CalculAngle
  (return (/ (Class|KismetMathLibrary|DegAcos (Math|Vector|DotProduct (Math|Vector|GetForwardVector (Variables|/Script/Engine.Character|GetCapsuleComponent (Variables|Default|GetPlayer))) (Math|Vector|GetForwardVector (Math|Conversions|RotationFromXVector (Math|Vector|GetForwardVector (Variables|Default|GetTextRender)))))) 1.8e+02)))