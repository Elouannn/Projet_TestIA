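; BP_Spawner is a one-shot enemy spawner triggered when the player character enters its box.
; It spawns EnnemisToSpawn BP_Ennemi actors, one per tick, at random reachable navmesh points within a fixed radius around itself.
; Each spawn is stored in SpawnedEnnemis, and the finished list is passed to the player via SetEnnemiListe.
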(event OnComponentBeginOverlap(Box)
  (params (OverlappedComponent :type Primitive%20Component%20Object%20Reference) (OtherActor :type Actor%20Object%20Reference) (OtherComp :type Primitive%20Component%20Object%20Reference) (OtherBodyIndex :type Integer) (bFromSweep :type Boolean) (SweepResult :type Hit%20Result%20Structure%20%28by%20ref%29))
  (bind _asbp_third_person_character (Utilities|Casting|CastToBP_ThirdPersonCharacter OtherActor))
  (Variables|Default|SetPlayer _asbp_third_person_character)
  (Utilities|FlowControl|DoOnce false
    (:Completed
      (Variables|Default|SetEnnemisSpawned 0)
      (if (< (Variables|Default|GetEnnemisSpawned) (Variables|Default|GetEnnemisToSpawn)) :!label _label
        (bind _returnvalue (Game|SpawnActorfromClass "/Game/Ennemis/BP_Ennemi.BP_Ennemi_C" (Math|Transform|MakeTransform (.RandomLocation (AI|Navigation|GetRandomReachablePointinRadius (Transformation|GetActorLocation) 3e+02 0 0)) "0, 0, 0" "1.000000,1.000000,1.000000") "AdjustIfPossibleButAlwaysSpawn" "MultiplyWithRoot" 0 0))
        (Utilities|Array|Add (Variables|Default|GetSpawnedEnnemis) _returnvalue)
        (Variables|Default|SetEnnemisSpawned (+ (Variables|Default|GetEnnemisSpawned) 1))
        (Utilities|FlowControl|DelayUntilNextTick)
        (goto _label)
        (else
          (Default|SetEnnemiListe (Variables|Default|GetPlayer) (Variables|Default|GetSpawnedEnnemis)))))))

(fn ConstructionScript)